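; BP_TestInteractableActor is a test interactable actor that logs who interacted with it and then destroys itself.
; Each Tick it copies the FocusWidget component's TimeRemaining into the Amount of its WBP_InteractionFocus widget.
; The Interact event prints the interacting actor and whether it runs with authority, then destroys the actor without gating on that check.
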(event `self.ReceiveBeginPlay`
  (`parent.ReceiveBeginPlay`))

(event `self.ReceiveTick`
  (params (DeltaSeconds :type "Float (single-precision)"))
  (bind _focuswidget (`self.FocusWidget`))
  (`parent.ReceiveTick` DeltaSeconds)
  (bind _aswbp_test_focus (cast `/Game/Blueprints/Interaction/WBP_InteractionFocus` (`WidgetComponent.GetWidget` _focuswidget)))
  (set `/Game/Blueprints/Interaction/WBP_InteractionFocus.Amount` (`FocusWidget.TimeRemaining` _focuswidget) _aswbp_test_focus))

(event `InteractionInterface.Interact`
  (params (OtherActor :type "Actor Object Reference"))
  (`KismetSystemLibrary.PrintString` (`KismetTextLibrary.Conv_TextToString` (`|FormatText` "Other Actor: {y} interacted with {x} \n" OtherActor self)))
  (`KismetSystemLibrary.PrintString` (`KismetStringLibrary.Conv_BoolToString` (`self.HasAuthority`)))
  (`self.K2_DestroyActor`))

(fn `UserConstructionScript`)
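; Test interactable actor that destroys itself when another actor interacts with it.
; The Interact event prints the interacting actor and itself, then whether it has network authority, before destroying the actor.
; The construction script writes InteractionDuration to a text render component, so the duration is visible on the actor.
; BeginPlay and Tick only call their parent versions.
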(event `self.ReceiveBeginPlay`
  (`parent.ReceiveBeginPlay`))

(event `self.ReceiveTick`
  (params (DeltaSeconds :type "Float (single-precision)"))
  (`parent.ReceiveTick` 0.0))

(event `InteractionInterface.Interact`
  (params (OtherActor :type "Actor Object Reference"))
  (`KismetSystemLibrary.PrintString` (`KismetTextLibrary.Conv_TextToString` (`|FormatText` "Other Actor: {y} interacted with {x} \n" OtherActor self)))
  (`KismetSystemLibrary.PrintString` (`KismetStringLibrary.Conv_BoolToString` (`self.HasAuthority`)))
  (`self.K2_DestroyActor`))

(fn `UserConstructionScript`
  (`TextRenderComponent.K2_SetText` (`self.TextRender`) (`KismetTextLibrary.Conv_DoubleToText` (`self.InteractionDuration`) "HalfToEven")))
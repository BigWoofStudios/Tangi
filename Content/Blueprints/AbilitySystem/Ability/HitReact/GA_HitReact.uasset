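; GA_HitReact is a gameplay ability for hit reactions, still unfinished.
; On activation it applies a gameplay effect to the owner, stores the handle and plays a montage, ending when playback completes, is interrupted or cancelled.
; Fetching the montage from the combat interface is only a TODO and debug print, so the montage variable is set to None.
; Ending the ability removes the effect by handle and clears both variables.
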(event `self.K2_ActivateAbility`
  ;[1 1 1] TODO: Get the hit react montage
  (`KismetSystemLibrary.PrintString` "Get hit react montage from combat interface")
  (`/Engine/EditorBlueprintResources/StandardMacros.IsValid` null
    (:`Is Valid`
      (set `self.AM_HitReact` null)
      (bind _returnvalue (`self.BP_ApplyGameplayEffectToOwner` null))
      (set `self.GE_HitReact` _returnvalue)
      (`AbilityTask_PlayMontageAndWait.CreatePlayMontageAndWaitProxy` "None" (`self.AM_HitReact`)
        (:`OnCompleted`
          _)
        (:`OnInterrupted`
          _)
        (:`OnCancelled`
          _))
      (`self.K2_EndAbility`))
    (:`Is Not Valid`
      (`self.K2_EndAbility`))))

(event `self.K2_OnEndAbility`
  (params (bWasCancelled :type Boolean))
  (`self.BP_RemoveGameplayEffectFromOwnerWithHandle` (`self.GE_HitReact`))
  (set `self.GE_HitReact` (struct))
  (set `self.AM_HitReact` null))
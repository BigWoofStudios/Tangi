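; Gameplay ability that lets a Tangi character sprint while the input is held.
; Activation adds a replicated sprinting tag, raises max walk speed and starts a looping timer that commits the ability cost while moving horizontally and not descending.
; Input release or a failed cost commit ends the ability, which clears the timer, restores the saved speed and removes the tag.
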(event `self.K2_ActivateAbility`
  (`self.ToggleIsSprintingTag` true)
  (`AbilityTask_WaitInputRelease.WaitInputRelease` false
    (:`then`
      (bind _astangi_character_base (cast `TangiCharacterBase` (`self.GetAvatarActorFromActorInfo`))
        (:`then`
          (bind _charactermovement (`Character.CharacterMovement` _astangi_character_base))
          (set `self.OG Speed` (`CharacterMovementComponent.MaxWalkSpeed` _charactermovement))
          (set `CharacterMovementComponent.MaxWalkSpeed` 1000.0 _charactermovement)
          (bind _returnvalue (`KismetSystemLibrary.K2_SetTimer` null "HandleSprintCost" 0.1 true))
          (set `self.Timer` _returnvalue))
        (:`CastFailed`
          (`self.K2_EndAbility`))))
    (:`OnRelease`
      (`self.K2_EndAbility`))))

(event `self.K2_OnEndAbility`
  (params (bWasCancelled :type Boolean))
  (`KismetSystemLibrary.K2_ClearAndInvalidateTimerHandle` (`self.Timer`))
  (bind _astangi_character_base (cast `TangiCharacterBase` (`self.GetAvatarActorFromActorInfo`)))
  (set `CharacterMovementComponent.MaxWalkSpeed` (`self.OG Speed`) (`Character.CharacterMovement` _astangi_character_base))
  (`self.ToggleIsSprintingTag` false))

(fn `GetShouldCommit`
  (returns (ReturnValue :type Boolean))
  (bind _returnvalue (`Actor.GetVelocity` (`self.GetAvatarActorFromActorInfo`)))
  (return (and (> (`KismetMathLibrary.VSizeXY` _returnvalue) 3.0) (>= (.z _returnvalue) 0.0))))

(fn `HandleSprintCost`
  (if (`self.GetShouldCommit`)
    (bind _returnvalue (`self.K2_CommitAbilityCost` false))
    (if (not _returnvalue)
      (`self.K2_EndAbility`))))

(fn `ToggleIsSprintingTag`
  (params (On :type Boolean))
  (locals (IsSprintTagContainer :type "GameplayTagContainer Structure" :default (struct :`GameplayTags` (struct :`(TagName` "Status.IsSprinting")))))
  (if On
    (bind _returnvalue (message `GameplayTagAssetInterface.HasMatchingGameplayTag` (`self.GetAvatarActorFromActorInfo`) (struct :`TagName` "Status.IsSprinting")))
    (if (not _returnvalue)
      (`AbilitySystemBlueprintLibrary.AddLooseGameplayTags` (`self.GetAvatarActorFromActorInfo`) (`local.IsSprintTagContainer`) true))
    (else
      (`AbilitySystemBlueprintLibrary.RemoveLooseGameplayTags` (`self.GetAvatarActorFromActorInfo`) (`local.IsSprintTagContainer`) true))))
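; GA_MeleeAttack is a gameplay ability that plays the avatar's melee attack montage and deals damage to the targets it hits.
; It waits for a montage gameplay event, then calls CauseDamage on targets that implement CombatInterface and are not already in HitActors.
; A rejected target, missing montage, or montage completion, interruption or cancellation ends the ability, and ending clears HitActors.
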(event `self.K2_ActivateAbility`
  (bind _returnvalue (message `CombatInterface.GetMeleeAttackMontage` (`self.GetAvatarActorFromActorInfo`)))
  (`/Engine/EditorBlueprintResources/StandardMacros.IsValid` _returnvalue
    (:`Is Valid`
      (`AbilityTask_PlayMontageAndWait.CreatePlayMontageAndWaitProxy` "None" _returnvalue
        (:`then`
          (bind (_asynctaskproxy _payload) (`AbilityTask_WaitGameplayEvent.WaitGameplayEvent` (struct :`TagName` "Gameplay.Event.Montage.ActivateAbility") null)
            (:`EventReceived`
              (bind (_bshouldcausedamage _targetactor) (`self.ShouldCauseDamage` _payload))
              (if _bshouldcausedamage
                (`BlueprintSetLibrary.Set_Add` (`self.HitActors`) _targetactor)
                (`self.CauseDamage` _targetactor)
                (else
                  (`self.K2_EndAbility`))))))
        (:`OnCompleted`
          (`self.K2_EndAbility` :!label _label))
        (:`OnInterrupted`
          (goto _label))
        (:`OnCancelled`
          (goto _label))))
    (:`Is Not Valid`
      (`self.K2_EndAbility`))))

(event `self.K2_OnEndAbility`
  (params (bWasCancelled :type Boolean))
  (`BlueprintSetLibrary.Set_Clear` (`self.HitActors`)))

(fn `ShouldCauseDamage`
  (params (GameplayEventData :type "GameplayEventData Structure (by ref)"))
  (returns (bShouldCauseDamage :type Boolean) (TargetActor :type "Actor Object Reference"))
  (bind ((`Target` _target)) (break `GameplayEventData` GameplayEventData))
  (return (and (not (`BlueprintSetLibrary.Set_Contains` (`self.HitActors`) _target)) (`KismetSystemLibrary.DoesImplementInterface` _target "/Script/Tangi.CombatInterface")) _target))